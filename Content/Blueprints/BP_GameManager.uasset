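; Game manager that runs turn-based combat between the player and a set of enemies.
; On begin play it shuffles player and enemies into a turn order, starts the first turn and creates the turn order HUD.
; NextTurn cycles through the list, starting each character's turn and updating the HUD.
; RemoveCharacter adjusts the turn index and shows game over when the player is removed or one character remains.
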(event EventBeginPlay
  (CallFunction|FindTurnOrder)
  ;[1 1 1] Display Turn Order UI
  (bind _returnvalue (UserInterface|CreateWidget "/Game/UI/UI_TurnOrder.UI_TurnOrder_C"))
  (bind _output_get (Variables|Default|SetturnOrderHUD _returnvalue))
  (UserInterface|Viewport|AddtoViewport _output_get 0)
  (Default|UpdateTurnUI (Variables|Default|GetturnOrderHUD) (Variables|Default|GetcurrentTurn) (Variables|Default|GetturnOrder)))

(event Collision|EventActorBeginOverlap
  (params (OtherActor :type Actor%20Object%20Reference)))

(event EventTick
  (params (DeltaSeconds :type Float%20%28single-precision%29)))

(fn ConstructionScript)

(fn NextTurn
  (bind _result (Math|Integer|IncrementInt (Variables|Default|GetcurrentTurn))
    (:%20%20
      ;[1 1 1] Loop Turn Order
      (if (>= _result (Utilities|Array|Length (Variables|Default|GetturnOrder)))
        (Variables|Default|SetcurrentTurn 0))
      ;[1 1 1] Activate Next Character
      (Default|StartTurn (Utilities|Array|Get(acopy) (Variables|Default|GetturnOrder) (Variables|Default|GetcurrentTurn)))
      (Default|UpdateTurnUI (Variables|Default|GetturnOrderHUD) (Variables|Default|GetcurrentTurn) (Variables|Default|GetturnOrder)))))

(fn FindTurnOrder
  (Utilities|Array|Clear (Variables|Default|GetturnOrder))
  ;[1 1 1] Populate Turn Order List
  (Utilities|Array|Add (Variables|Default|GetturnOrder) (Variables|Default|Getplayer))
  (Utilities|Array|AppendArray (Variables|Default|GetturnOrder) (Variables|Default|Getenemies))
  ;[1 1 1] Randomise Turn Order
  (Utilities|Array|Shuffle (Variables|Default|GetturnOrder))
  ;[1 1 1] Set First Character Active
  (Default|StartTurn (Utilities|Array|Get(acopy) (Variables|Default|GetturnOrder))))

(fn RemoveCharacter
  (params (character :type BP%20Character%20Object%20Reference))
  ;[1 1 1] If killed character is before current in turn order, adjust turn index
  (if (< (Utilities|Array|FindItem (Variables|Default|GetturnOrder) character) (Variables|Default|GetcurrentTurn))
    (Math|Integer|DecrementInt (Variables|Default|GetcurrentTurn)
      (:%20%20
        _)))
  (Utilities|Array|RemoveItem (Variables|Default|GetturnOrder) character)
  (Default|UpdateTurnUI (Variables|Default|GetturnOrderHUD) (Variables|Default|GetcurrentTurn) (Variables|Default|GetturnOrder))
  (if (or (== character (Variables|Default|Getplayer)) (<= (Utilities|Array|Length (Variables|Default|GetturnOrder)) 1))
    ;[1 1 1] Display Game Over Screen
    (bind _returnvalue (UserInterface|CreateWidget "/Game/UI/UI_GameOver.UI_GameOver_C"))
    (UserInterface|Viewport|AddtoViewport _returnvalue 0)
    (Variables|/Script/Engine.PlayerController|SetbShowMouseCursor (Game|GetPlayerController 0) true)))