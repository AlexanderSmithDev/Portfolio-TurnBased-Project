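; Base character for turn-based combat, tracking health, movement and attack allowances, with turns handed on through the GameManager.
; Each turn start refills movement and attacks, while ending a turn stops the character and advances the turn order.
; Attacks roll against accuracy that falls with distance, stays above zero within range and is zero beyond it.
; Damage fires a Damaged event or, at zero health, removes the character from the GameManager and destroys it.
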(event Custom|Damaged)

(event Custom|Killed
  (Actor|DestroyActor))

(event EventBeginPlay)

(event Collision|EventActorBeginOverlap
  (params (OtherActor :type Actor%20Object%20Reference)))

(event EventTick
  (params (DeltaSeconds :type Float%20%28single-precision%29)))

(fn ConstructionScript
  (Variables|Default|SetcurrentHealth (Variables|Default|GetmaxHealth)))

(fn StartTurn
  (Variables|Default|SetcharacterActive true)
  (Variables|Default|SetremainingMovement (Variables|Default|GetmoveLimit))
  (Variables|Default|SetattacksRemaining (Variables|Default|GetattackLimit)))

(fn EndTurn
  (Variables|Default|SetcharacterActive false)
  (Variables|Default|Setvelocity "0, 0, 0")
  (Default|NextTurn (Variables|Default|GetgameManager)))

(fn TakeDamage
  (params (damageTaken :type Integer))
  ;[1 1 1] Take Damage
  (Variables|Default|SetcurrentHealth (- (Variables|Default|GetcurrentHealth) damageTaken))
  (if (<= (Variables|Default|GetcurrentHealth) 0)
    ;[1 1 1] Die
    (CallFunction|KillCharacter)
    (CallFunction|Killed)
    (else
      (CallFunction|Damaged))))

(fn KillCharacter
  ;[1 1 1] Remove from Turn Order
  (Default|RemoveCharacter (Variables|Default|GetgameManager) self))

(fn Attack
  (params (attackTarget :type BP%20Character%20Object%20Reference%20%28by%20ref%29))
  (Math|Integer|DecrementInt (Variables|Default|GetattacksRemaining)
    (:%20%20
      ;[1 1 1] Determine if Attack Hits
      (bind _accuracy (CallFunction|CalculateAccuracy attackTarget))
      (if (<= (* (Math|Random|RandomFloat) 1e+02) _accuracy)
        (CallFunction|TakeDamage attackTarget (Variables|Default|GetattackDamage))))))

(fn CalculateAccuracy
  (params (accuracyTarget :type BP%20Character%20Object%20Reference%20%28by%20ref%29))
  ;[1 1 1] If within range, Accuracy = Percentage of Max Accuracy, based on Distance (low Distance = high Accuracy), with non-zero minimum Accuracy
  (LocalVariables|Setdistance (Math|Vector|Distance(Vector) (Transformation|GetWorldLocation (Variables|/Script/Engine.Actor|GetRootComponent accuracyTarget)) (Transformation|GetWorldLocation (Variables|Transformation|GetRootComponent))))
  (if (> (LocalVariables|Getdistance) (Variables|Default|GetattackRange))
    (return 0.0)
    (else
      (return (- (Variables|Default|GetattackMaxAccuracy) (* (Variables|Default|GetattackMaxAccuracy) (/ (/ (LocalVariables|Getdistance) 1e+02) (+ (/ (Variables|Default|GetattackRange) 1e+02) 1.0))))))))