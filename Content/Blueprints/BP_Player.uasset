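; Player-controlled character for a turn-based shooter, handling input, movement, aiming, attacks and HUD updates while its turn is active.
; Tick integrates a custom velocity with deceleration and a swept move, deducting distance from the turn's movement budget.
; A manual orbit camera eases toward its target and watches the current turn's character, or switches to over-the-shoulder aim, where a line trace picks the enemy for accuracy display and attack.
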(event Input|EnhancedActionEvents|EnhancedInputActionIA_Move
  (params (ActionValue :type Vector%202D%20Structure) (ElapsedSeconds :type Float%20%28double-precision%29) (TriggeredSeconds :type Float%20%28double-precision%29) (InputAction :type Input%20Action%20Object%20Reference :default "/Game/Input/IA_Move.IA_Move"))
  (bind (_x _y) (Math|Vector2D|BreakVector2D ActionValue))
  (bind _camera (Variables|Default|GetCamera))
  (bind _camera_2 (Variables|Default|GetCamera))
  (bind _returnvalue (Math|Vector|GetForwardVector _camera))
  (bind _returnvalue_2 (Math|Vector|GetRightVector _camera_2))
  (bind (_x_2 _y_2) (Math|Vector|BreakVector _returnvalue_2))
  (bind (_x_3 _y_3) (Math|Vector|BreakVector _returnvalue))
  (if (and (Variables|Default|GetcharacterActive) (not (Variables|Default|GetplayerAiming)))
    (if (> (Variables|Default|GetremainingMovement) 0.0)
      ;[1 1 1] Apply Acceleration
      (Variables|Default|Setvelocity (+ (Variables|Default|Getvelocity) (* (Math|Vector2D|Normalize2D (Math|Vector2D|MakeVector2D _x_2 _y_2)) (Variables|Default|Getacceleration) (Utilities|Time|GetWorldDeltaSeconds) _x) (* (Math|Vector2D|Normalize2D (Math|Vector2D|MakeVector2D _x_3 _y_3)) _y (Variables|Default|Getacceleration) (Utilities|Time|GetWorldDeltaSeconds))))
      ;[1 1 1] Player Face Camera Direction
      (Class|Actor|AddActorWorldRotation (Math|Rotator|MakeRotator 0.0 0.0 (Variables|Default|GetcameraHorizAngle)))
      ;[1 1 1] Reset Camera Rotation / Position
      (Variables|Default|SetcameraHorizAngle 0.0)
      (CallFunction|FindCameraTargetPos))))

(event Input|EnhancedActionEvents|EnhancedInputActionIA_Look
  (params (ActionValue :type Vector%202D%20Structure) (ElapsedSeconds :type Float%20%28double-precision%29) (TriggeredSeconds :type Float%20%28double-precision%29) (InputAction :type Input%20Action%20Object%20Reference :default "/Game/Input/IA_Look.IA_Look"))
  (bind (_x _y) (Math|Vector2D|BreakVector2D ActionValue))
  (if (Variables|Default|GetcharacterActive)
    (Utilities|FlowControl|Sequence
      (:then_0
        ;[1 1 1] Calculate Camera Delta
        (Variables|Default|SetcameraHorizDelta (* (Variables|Default|GetcameraSensitivity) (Utilities|Time|GetWorldDeltaSeconds) _x))
        (Variables|Default|SetcameraVertDelta (* (Variables|Default|GetcameraSensitivity) (Utilities|Time|GetWorldDeltaSeconds) _y)))
      (:then_1
        (if (Variables|Default|GetplayerAiming)
          ;[1 1 1] Rotate Character When Aiming
          (Class|Actor|AddActorWorldRotation (Math|Rotator|MakeRotator 0.0 0.0 (Variables|Default|GetcameraHorizDelta)))
          ;[1 1 1] Camera Aim Vertical Rotation
          (bind _output_get (Variables|Default|SetcameraVertAngle (Math|Float|Clamp(Float) (+ (Variables|Default|GetcameraVertDelta) (Variables|Default|GetcameraVertAngle)) -7e+01 7e+01)))
          (Transformation|SetRelativeRotation (Variables|Default|GetCamera) (Math|Rotator|MakeRotator 0.0 _output_get 0.0) false false)
          (else
            ;[1 1 1] Apply Camera Rotation
            (Variables|Default|SetcameraHorizAngle (+ (Variables|Default|GetcameraHorizDelta) (Variables|Default|GetcameraHorizAngle)))
            (Variables|Default|SetcameraVertAngle (Math|Float|Clamp(Float) (+ (Variables|Default|GetcameraVertDelta) (Variables|Default|GetcameraVertAngle)) -7e+01 7e+01))
            ;[1 1 1] Set Camera Target Position
            (CallFunction|FindCameraTargetPos)))))))

(event Input|EnhancedActionEvents|EnhancedInputActionIA_EndTurn
  (params (ActionValue :type Boolean) (ElapsedSeconds :type Float%20%28double-precision%29) (TriggeredSeconds :type Float%20%28double-precision%29) (InputAction :type Input%20Action%20Object%20Reference :default "/Game/Input/IA_EndTurn.IA_EndTurn"))
  (:Started
    (if (Variables|Default|GetcharacterActive)
      (if (Variables|Default|GetplayerAiming)
        (CallFunction|ToggleAim))
      ;[1 1 1] End Player Turn
      (CallFunction|EndTurn))))

(event Input|EnhancedActionEvents|EnhancedInputActionIA_Aim
  (params (ActionValue :type Boolean) (ElapsedSeconds :type Float%20%28double-precision%29) (TriggeredSeconds :type Float%20%28double-precision%29) (InputAction :type Input%20Action%20Object%20Reference :default "/Game/Input/IA_Aim.IA_Aim"))
  (:Started
    (if (Variables|Default|GetcharacterActive)
      (CallFunction|ToggleAim))))

(event Input|EnhancedActionEvents|EnhancedInputActionIA_Attack
  (params (ActionValue :type Boolean) (ElapsedSeconds :type Float%20%28double-precision%29) (TriggeredSeconds :type Float%20%28double-precision%29) (InputAction :type Input%20Action%20Object%20Reference :default "/Game/Input/IA_Attack.IA_Attack"))
  (if (Math|Boolean|ANDBoolean (Variables|Default|GetcharacterActive) (Variables|Default|GetplayerAiming) (Utilities|IsValid (Variables|Default|GetfocusedEnemy)) (> (Variables|Default|GetattacksRemaining) 0))
    (CallFunction|Attack (Variables|Default|GetfocusedEnemy))
    (Default|UpdateAttackUI (Variables|Default|GetplayerHUD) (Variables|Default|GetattacksRemaining))
    (Variables|Default|SetcharacterActive false)
    (Animation|Montage|PlayMontage (Variables|Default|GetcharacterLargeMale) "/Game/Animations/Montages/Male/MaleShoot.MaleShoot"
      (:OnCompleted
        (Variables|Default|SetcharacterActive true)))))

(event EventBeginPlay
  ;[1 1 1] Initialise Input
  (bind _asplayer_controller (Utilities|Casting|CastToPlayerController (Pawn|GetController)))
  (Utilities|IsValid (PlayerController|LocalPlayerSubsystems|GetEnhancedInputLocalPlayerSubsystem _asplayer_controller)
    (:Is%20Valid
      (Input|AddMappingContext (PlayerController|LocalPlayerSubsystems|GetEnhancedInputLocalPlayerSubsystem _asplayer_controller) "/Game/Input/IMC_Player.IMC_Player" 0 "(bIgnoreAllPressedKeysUntilRelease=True,bForceImmediately=False,bNotifyUserSettings=False)")
      ;[1 1 1] Display Player UI
      (bind _returnvalue (UserInterface|CreateWidget "/Game/UI/UI_PlayerHUD.UI_PlayerHUD_C"))
      (bind _output_get (Variables|Default|SetplayerHUD _returnvalue))
      (UserInterface|Viewport|AddtoViewport _output_get 0)
      (Variables|Default|SetcameraTargetPos (Variables|/Script/Engine.SceneComponent|GetRelativeLocation (Variables|Default|GetCamera))))))

(event Collision|EventActorBeginOverlap
  (params (OtherActor :type Actor%20Object%20Reference)))

(event EventTick
  (params (DeltaSeconds :type Float%20%28single-precision%29))
  (bind _gamemanager (Variables|Default|GetgameManager))
  (bind _camera (Variables|Default|GetCamera))
  (bind _returnvalue (Transformation|GetWorldLocation _camera))
  ;[1 1 1] Deceleration
  (Variables|Default|Setvelocity (- (Variables|Default|Getvelocity) (* (Variables|Default|Getvelocity) (Variables|Default|Getdeceleration) (Utilities|Time|GetWorldDeltaSeconds))))
  ;[1 1 1] Velocity Limit
  (if (> (Class|KismetMathLibrary|VSizeXYSquared (Variables|Default|Getvelocity)) (Math|Float|Square (Variables|Default|GetmaxVelocity)))
    (Variables|Default|Setvelocity (* (Class|KismetMathLibrary|VectorNormal2D (Variables|Default|Getvelocity) 0.0001) (Variables|Default|GetmaxVelocity))))
  ;[1 1 1] Apply Movement
  (Transformation|SetActorLocation (+ (Transformation|GetActorLocation) (* (Variables|Default|Getvelocity) (Utilities|Time|GetWorldDeltaSeconds))) true false)
  ;[1 1 1] Track Spent Movement
  (Variables|Default|SetremainingMovement (- (Variables|Default|GetremainingMovement) (Math|Vector|VectorLengthXY (* (Variables|Default|Getvelocity) (Utilities|Time|GetWorldDeltaSeconds)))))
  (Default|UpdateMovementUI (Variables|Default|GetplayerHUD) (Variables|Default|GetremainingMovement) (Variables|Default|GetmoveLimit))
  (Utilities|FlowControl|Sequence
    (:then_0
      ;[1 1 1] Camera Drag
      (Transformation|SetWorldLocation (Variables|Default|GetCamera) (- (Transformation|GetWorldLocation (Variables|Default|GetCamera)) (* (Variables|Default|Getvelocity) (Variables|Default|GetcameraDrag) (Utilities|Time|GetWorldDeltaSeconds))) false false)
      ;[1 1 1] Camera Move
      (if (> (Class|KismetMathLibrary|VectorDistanceSquared (Variables|/Script/Engine.SceneComponent|GetRelativeLocation (Variables|Default|GetCamera)) (Variables|Default|GetcameraTargetPos)) 25.0)
        (Transformation|AddRelativeLocation (Variables|Default|GetCamera) (* (- (Variables|Default|GetcameraTargetPos) (Variables|/Script/Engine.SceneComponent|GetRelativeLocation (Variables|Default|GetCamera))) (Variables|Default|GetcameraSpeed) (Utilities|Time|GetWorldDeltaSeconds)) false false))
      (if (Variables|Default|GetplayerAiming)
        ;[1 1 1] Check Aim Target
        (bind _outhit (Collision|LineTraceByChannel _returnvalue (+ _returnvalue (* (Math|Vector|GetForwardVector (Variables|Default|GetCamera)) 1e+05)) "TraceTypeQuery1" false 0 "None"))
        (bind _asbp_character (Utilities|Casting|CastToBP_Character (.HitActor (Collision|BreakHitResult _outhit)))
          (:then
            _)
          (:CastFailed
            _))
        (bind _output_get (Variables|Default|SetfocusedEnemy _asbp_character))
        (if (Utilities|IsValid (Variables|Default|GetfocusedEnemy))
          (bind _accuracy (CallFunction|CalculateAccuracy (Variables|Default|GetfocusedEnemy)))
          (Default|UpdateFocusedEnemy (Variables|Default|GetplayerHUD) _output_get (Math|Float|Round _accuracy))
          (else
            (Default|UpdateFocusedEnemy (Variables|Default|GetplayerHUD))))
        (else
          ;[1 1 1] Camera Focus on Player
          (Transformation|SetWorldRotation (Variables|Default|GetCamera) (Math|Rotator|FindLookatRotation (Transformation|GetWorldLocation (Variables|Default|GetCamera)) (+ (Transformation|GetWorldLocation (Variables|/Game/Blueprints/BP_Character.BP_Character_C|GetCapsule (Utilities|Array|Get(acopy) (Variables|/Game/Blueprints/BP_GameManager.BP_GameManager_C|GetturnOrder _gamemanager) (Variables|/Game/Blueprints/BP_GameManager.BP_GameManager_C|GetcurrentTurn _gamemanager)))) "0.000000,0.000000,85.000000")) false false))))))

(event EventDamaged
  (Default|UpdateHealthUI (Variables|Default|GetplayerHUD) (Variables|Default|GetcurrentHealth) (Variables|Default|GetmaxHealth))
  (Animation|Montage|PlayMontage (Variables|Default|GetcharacterLargeMale) "/Game/Animations/Montages/Male/MaleHurt.MaleHurt"))

(event EventKilled
  (Animation|Montage|PlayMontage (Variables|Default|GetcharacterLargeMale) "/Game/Animations/Montages/Male/MaleDie.MaleDie"
    (:OnCompleted
      (Actor|DestroyActor))))

(fn ConstructionScript)

(fn FindCameraTargetPos
  (Variables|Default|SetcameraTargetPos (Math|Vector|MakeVector (* -1.0 (Math|Trig|Cos(Degrees) (Variables|Default|GetcameraHorizAngle)) (Math|Trig|Cos(Degrees) (Variables|Default|GetcameraVertAngle)) (Variables|Default|GetcameraDistance)) (* -1.0 (Math|Trig|Sin(Degrees) (Variables|Default|GetcameraHorizAngle)) (Math|Trig|Cos(Degrees) (Variables|Default|GetcameraVertAngle)) (Variables|Default|GetcameraDistance)) (+ (* -1.0 (Math|Trig|Sin(Degrees) (Variables|Default|GetcameraVertAngle)) (Variables|Default|GetcameraDistance)) (Variables|Default|GetBaseEyeHeight)))))

(fn ToggleAim
  ;[1 1 1] Toggle Aim
  (Variables|Default|SetplayerAiming (not (Variables|Default|GetplayerAiming)))
  (if (Variables|Default|GetplayerAiming)
    (Class|Actor|AddActorWorldRotation (Math|Rotator|MakeRotator 0.0 0.0 (Variables|Default|GetcameraHorizAngle)))
    ;[1 1 1] Reset Camera Rotation When Aiming
    (Variables|Default|SetcameraHorizAngle 0.0)
    (Variables|Default|SetcameraVertAngle 0.0)
    (Transformation|SetRelativeRotation (Variables|Default|GetCamera) "0, 0, 0" false false)
    ;[1 1 1] Move Camera To Aim Position
    (Variables|Default|SetcameraTargetPos (Math|Vector|MakeVector -5e+01 5e+01 (Variables|Default|GetBaseEyeHeight)))
    (Widget|SetVisibility (Variables|/Game/UI/UI_PlayerHUD.UI_PlayerHUD_C|GetCrosshair (Variables|Default|GetplayerHUD)) "Visible")
    (else
      (bind _output_get (Variables|Default|SetfocusedEnemy 0))
      (Default|UpdateFocusedEnemy (Variables|Default|GetplayerHUD) _output_get)
      (CallFunction|FindCameraTargetPos)
      (Widget|SetVisibility (Variables|/Game/UI/UI_PlayerHUD.UI_PlayerHUD_C|GetCrosshair (Variables|Default|GetplayerHUD)) "Collapsed"))))

(fn StartTurn
  (|CallParentFunction)
  (if (Utilities|IsValid (Variables|Default|GetplayerHUD))
    (Default|UpdateMovementUI (Variables|Default|GetplayerHUD) (Variables|Default|GetremainingMovement) (Variables|Default|GetmoveLimit))
    (Default|UpdateAttackUI (Variables|Default|GetplayerHUD) (Variables|Default|GetattacksRemaining))
    (Default|UpdateHealthUI (Variables|Default|GetplayerHUD) (Variables|Default|GetcurrentHealth) (Variables|Default|GetmaxHealth))))