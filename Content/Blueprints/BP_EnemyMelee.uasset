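; BP_EnemyMelee is a turn-based melee enemy that reacts to damage and death but currently makes no attack.
; StartTurn runs the parent logic, then EnemyBehaviour, which only waits a few seconds before ending the turn.
; Damaged plays the FemaleHurt montage, and Killed plays FemaleDie, destroying the actor once that montage completes.
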(event Custom|Enemy%20Behaviour
  (Utilities|FlowControl|Delay 3.0)
  (CallFunction|EndTurn))

(event EventBeginPlay)

(event Collision|EventActorBeginOverlap
  (params (OtherActor :type Actor%20Object%20Reference)))

(event EventTick
  (params (DeltaSeconds :type Float%20%28single-precision%29)))

(event EventDamaged
  (Animation|Montage|PlayMontage (Variables|Default|GetSkeletalMesh) "/Game/Animations/Montages/Female/FemaleHurt.FemaleHurt"))

(event EventKilled
  (Animation|Montage|PlayMontage (Variables|Default|GetSkeletalMesh) "/Game/Animations/Montages/Female/FemaleDie.FemaleDie"
    (:OnCompleted
      (Actor|DestroyActor))))

(fn ConstructionScript)

(fn StartTurn
  (|CallParentFunction)
  (CallFunction|EnemyBehaviour))